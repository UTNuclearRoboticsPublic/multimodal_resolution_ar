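; Base actor for mixed-reality map representations that can be saved as Azure Spatial Anchors, with a child menu showing status.
; Saving packs ID, rotation and scale into properties and requests an anchor from MRGameMode.
; Deleting unpins the root component; DeleteDatabaseEntry only destroys the actor.
; Menu setup, button binding and detected-item spawning logic are disconnected, so the save and delete handlers are never bound here.
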(event `self.ReceiveBeginPlay`
  ;[1 1 1] Event Begin Play
  (`self.Setup Anchor Menu`))

(event `Setup Anchor Menu`
  ;[1 1 1] Setup Anchor Menu: Call Create Anchor if "Save" Button is Pushed, Call Delete Anchor if "Delete" Button is Pushed
)

(event `SaveButtonPressedHandler`
  (params (Button :type "UxtPressableButtonComponent Object Reference") (Pointer :type "UxtPointerComponent Object Reference"))
  ;[1 1 1] Setup Anchor Menu: Call Create Anchor if "Save" Button is Pushed, Call Delete Anchor if "Delete" Button is Pushed
  (`self.Create Anchor`))

(event `DeleteButtonPressedHandler`
  (params (Button :type "UxtPressableButtonComponent Object Reference") (Pointer :type "UxtPointerComponent Object Reference"))
  ;[1 1 1] Setup Anchor Menu: Call Create Anchor if "Save" Button is Pushed, Call Delete Anchor if "Delete" Button is Pushed
  (`self.Delete Anchor`))

(event `Create Anchor`
  ;[1 1 1] Create Anchor Event: Change Anchor Status Test and Call "Request Anchor Creation"
  (`KismetSystemLibrary.PrintString` (`KismetStringLibrary.Concat_StrStr` (`self.Representation ID`) " Wants To Create Anchor. Anchor Details  \n**************************************************************************************************") false)
  (`self.SetStatusText` "Saving...")
  (`self.Request Anchor Creation` 860000.0)
  (`KismetSystemLibrary.PrintString` "  \n**************************************************************************************************"))

(event `Delete Anchor`
  ;[1 1 1] Delete Anchor
  (`KismetSystemLibrary.PrintString` (`KismetStringLibrary.Concat_StrStr` (`self.Representation ID`) " wants to delete anchor") false)
  (`self.SetStatusText` "Deleting...")
  (`ARBlueprintLibrary.UnpinComponent` (`self.DefaultSceneRoot`)))

(event `self.ReceiveTick`
  (params (DeltaSeconds :type "Float (single-precision)")))

(event `ListenForDetectedItemMessages`
  (`KismetSystemLibrary.PrintString` "*********************SETTING UP**********************")
  (bind _returnvalue (`RobofleetBPFunctionLibrary.GetClientReference`)))

(event `OnDetectedItemMsgReceived`
  (params (DetectedItemUid :type String)))

(fn `Request Anchor Creation`
  (params (Lifetime :type "Float (double-precision)"))
  (bind _returnvalue (`self.GetTransform`))
  (bind _representation_properties (`self.Representation Properties`))
  (`|ExecutionSequence`
    (:`then_0`
      ;[1 1 1] Step 1: Create Represenation ID and Representation Properties Array
      (`BlueprintMapLibrary.Map_Add` _representation_properties "Representation ID" (`self.Representation ID`))
      (`BlueprintMapLibrary.Map_Add` _representation_properties "Rot.X" (`KismetStringLibrary.Conv_DoubleToString` (.roll (.rotation _returnvalue))))
      (`BlueprintMapLibrary.Map_Add` _representation_properties "Rot.Y" (`KismetStringLibrary.Conv_DoubleToString` (.pitch (.rotation _returnvalue))))
      (`BlueprintMapLibrary.Map_Add` _representation_properties "Rot.Z" (`KismetStringLibrary.Conv_DoubleToString` (.yaw (.rotation _returnvalue))))
      (`BlueprintMapLibrary.Map_Add` _representation_properties "Scale.X" (`KismetStringLibrary.Conv_DoubleToString` (.x (.scale _returnvalue))))
      (`BlueprintMapLibrary.Map_Add` _representation_properties "Scale.Y" (`KismetStringLibrary.Conv_DoubleToString` (.y (.scale _returnvalue))))
      (`BlueprintMapLibrary.Map_Add` _representation_properties "Scale.Z" (`KismetStringLibrary.Conv_DoubleToString` (.z (.scale _returnvalue))))
      (`BlueprintMapLibrary.Map_Keys` _representation_properties))
    (:`then_1`
      ;[1 1 1] Step 2: Take Represenation ID and Properties Array then
      ;
      ; Call "Create Azure Spatial Anchor" function from AugREGameModeMain
      (bind _asmrgame_mode (cast `/Game/Core/MRGameMode` (`GameplayStatics.GetGameMode`)))
      (`/Game/Core/MRGameMode.Create Azure Spatial Anchor` _asmrgame_mode (`self.DefaultSceneRoot`) Lifetime (`self.Representation ID`) (`self.Representation Properties`)))))

(fn `SetStatusText`
  (params (`Status Text` :type Text))
  (bind _asbp_representation_anchor_menu (cast `/Game/UI/BP_RepresentationAnchorMenu` (`ChildActorComponent.ChildActor` (`self.AnchorMenu`))))
  (bind _aswbp_representation_anchor_status (cast `/Game/UI/WBP_RepresentationAnchorStatus` (`WidgetComponent.GetWidget` (`/Game/UI/BP_RepresentationAnchorMenu.StatusWidget` _asbp_representation_anchor_menu))))
  (`TextBlock.SetText` (`/Game/UI/WBP_RepresentationAnchorStatus.Status` _aswbp_representation_anchor_status) `Status Text`))

(fn `UserConstructionScript`)