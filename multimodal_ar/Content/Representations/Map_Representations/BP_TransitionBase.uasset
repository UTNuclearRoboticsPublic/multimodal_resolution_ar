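; BP_TransitionBase is a base map representation for a transition, with an entry site and an exit site.
; Its anchor creation request adds both sites to the representation properties, then calls the parent implementation with the given lifetime.
; Play Transition Effects takes a head tracker and is an empty hook here.
; Every tick it draws the entry and exit boxes as debug boxes in distinct colors.
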(event `self.ReceiveTick`
  (params (DeltaSeconds :type "Float (single-precision)"))
  (bind _entry_box (`self.Entry Box`))
  (bind _exit_box (`self.Exit Box`))
  (`KismetSystemLibrary.DrawDebugBox` (`SceneComponent.K2_GetComponentLocation` _entry_box) (`BoxComponent.GetScaledBoxExtent` _entry_box) (struct :`R` 1.0 :`B` 0.129513 :`A` 1.0) (`SceneComponent.K2_GetComponentRotation` _entry_box) 0.0 2.0)
  (`KismetSystemLibrary.DrawDebugBox` (`SceneComponent.K2_GetComponentLocation` _exit_box) (`BoxComponent.GetScaledBoxExtent` _exit_box) (struct :`R` 1.0 :`G` 0.719175 :`B` 0.059654 :`A` 1.0) (`SceneComponent.K2_GetComponentRotation` _exit_box) 0.0 2.0))

(fn `Play Transition Effects`
  (params (`Head Tracker` :type "Object Object Reference")))

(fn `Request Anchor Creation`
  (params (Lifetime :type "Float (double-precision)"))
  (bind _representation_properties (`self.Representation Properties`))
  (`BlueprintMapLibrary.Map_Add` _representation_properties "Entry Site" (`self.Entry Site`))
  (`BlueprintMapLibrary.Map_Add` _representation_properties "Exit Site" (`self.Exit Site`))
  (`parent.Request Anchor Creation` Lifetime))

(fn `UserConstructionScript`)