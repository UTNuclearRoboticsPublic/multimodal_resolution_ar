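; BP_RoomBase is an anchorable map representation of a site, meant to host mobile representations of that site's Robofleet robots.
; When anchored, BeginPlay waits five seconds, requests a representation per robot, then binds detected-item messages to spawn image-sized menus near the user's head pose.
; SpawnMobileRepresentation and new-robot subscription are stubbed, their logic left disconnected.
; Anchor creation requests add the Site to the representation properties.
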(event `SetDebugOptions`
  (params (IsDebugPrintLog :type Boolean) (IsDebugPrintScreen :type Boolean))
  (set `self.IsDebugPrintScreen` IsDebugPrintScreen)
  (set `self.IsDebugPrintLog` IsDebugPrintLog))

(event `self.ReceiveBeginPlay`
  (bind _isdebugprintscreen (`self.IsDebugPrintScreen`))
  (bind _isdebugprintlog (`self.IsDebugPrintLog`))
  (`self.SetDebugOptions` true)
  (`self.Setup Anchor Menu`)
  ;[1 1 1] Event Begin Play: Mobile Represenation Spawn of All Existing Robots
  (`KismetSystemLibrary.PrintString` "Anchor Menu Created, Returning to BP_RoomBase" (`self.IsDebugPrintScreen`) (`self.IsDebugPrintLog`))
  (if (`self.IsAnchored`)
    (`KismetSystemLibrary.PrintString` (`KismetStringLibrary.Concat_StrStr` "Trying to Spawn Mobile Representation for ALL Robots at Site: " (`self.Site`)) _isdebugprintscreen _isdebugprintlog)
    (`KismetSystemLibrary.K2_SetTimerDelegate` (delegate `Wait2`) 5.0)
    (else
      (`KismetSystemLibrary.PrintString` "Room Base Not Anchored" _isdebugprintscreen _isdebugprintlog))))

(event `Wait2`
  ;[1 1 1] Event Begin Play: Mobile Represenation Spawn of All Existing Robots
  (bind _returnvalue (`RobofleetBPFunctionLibrary.GetAllRobotsAtSite` (`self.Site`)))
  (for _array_element _returnvalue
    (`KismetSystemLibrary.PrintString` (`KismetStringLibrary.Concat_StrStr` "Found: " _array_element ", Spawning Menu ...") (`self.IsDebugPrintScreen`) (`self.IsDebugPrintLog`))
    (`self.Spawn Mobile Representation` (`KismetMathLibrary.MakeTransform` (`self.K2_GetActorLocation`) (struct) (0.2 0.2 0.2)) "Undefined" _array_element))
  (`KismetSystemLibrary.PrintString` "Completed Loop Through All Robots at Site" (`self.IsDebugPrintScreen`) (`self.IsDebugPrintLog`))
  (`self.SetupOnNewRobotFoundOnRobofleet`)
  (`self.ListenForDetectedItems`))

(event `SetupOnNewRobotFoundOnRobofleet`
  ;[1 1 1] Spawn Menu if New Robot is found on Robofleet in the Room Base was Spawned
)

(event `OnNewRobotSeen`
  (params (RobotName :type String))
  ;[1 1 1] Spawn Menu if New Robot is found on Robofleet in the Room Base was Spawned
  (bind _returnvalue (`RobofleetBPFunctionLibrary.GetRobotLocationString` RobotName))
  (`KismetSystemLibrary.PrintString` (`KismetStringLibrary.Concat_StrStr` "[New Robot Seen: " RobotName "] Location: " _returnvalue) (`self.IsDebugPrintScreen`) (`self.IsDebugPrintLog`) (struct :`G` 0.66 :`B` 1.0 :`A` 1.0) 20.0)
  (if (`KismetStringLibrary.EqualEqual_StrStr` _returnvalue (`self.Site`))
    (`KismetSystemLibrary.PrintString` (`KismetStringLibrary.Concat_StrStr` "Spawning Menu for: " RobotName "...") (`self.IsDebugPrintScreen`) (`self.IsDebugPrintLog`))
    (`self.Spawn Mobile Representation` (`KismetMathLibrary.MakeTransform` (`self.K2_GetActorLocation`) (struct) (0.2 0.2 0.2)) "Undefined" RobotName)))

(event `ListenForDetectedItems`
  (bind _returnvalue (`RobofleetBPFunctionLibrary.GetClientReference`))
  (add `RobofleetBase.OnDetectedItemReceived` _returnvalue (delegate `OnMessageReceived`)))

(event `OnMessageReceived`
  (params (DetectedItemUid :type String) (frame_id :type String))
  (bind (_returnvalue_location _returnvalue_rotation) (`KismetMathLibrary.BreakTransform` (`UxtFunctionLibrary.GetHeadPose`)))
  (bind _returnvalue (`RobofleetBPFunctionLibrary.GetDetectedImageSize` DetectedItemUid))
  (`|SpawnActorFromClass` "/Game/UI/detected_item_menu/blueprints/BP_detected_item_menu.BP_detected_item_menu_C" (`KismetMathLibrary.MakeTransform` (+ _returnvalue_location (* (`KismetMathLibrary.GetForwardVector` _returnvalue_rotation) 80.0) (* (`KismetMathLibrary.GetRightVector` _returnvalue_rotation) -40.0) (* (`KismetMathLibrary.GetUpVector` _returnvalue_rotation) -40.0)) (`KismetMathLibrary.MakeRotator` 0.0 0.0 (+ (.yaw (.rotation (`UxtFunctionLibrary.GetHeadPose`))) 180.0)) (0.2 0.2 0.2)) "Undefined" "OverrideRootScale" self DetectedItemUid null (`KismetMathLibrary.FTrunc` (.y _returnvalue)) (`KismetMathLibrary.FTrunc` (.x _returnvalue)) null))

(fn `Request Anchor Creation`
  (params (Lifetime :type "Float (double-precision)"))
  (`BlueprintMapLibrary.Map_Add` (`self.Representation Properties`) "Site" (`self.Site`))
  (`parent.Request Anchor Creation` Lifetime))

(fn `Spawn Mobile Representation`
  (params (`Spawn Transform` :type "Transform Structure") (`Collision Handling Override` :type "ESpawnActorCollisionHandlingMethod Enum" :default "Undefined") (`Robot Name` :type String))
  (locals (TfNamespace :type String) (SpawnTransform :type "Transform Structure") (CollisionHandlingOverride :type "ESpawnActorCollisionHandlingMethod Enum") (AgentCallsign :type String)))

(fn `UserConstructionScript`)