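; Chatbot pawn prototype that turns "here" and "there" navigation commands into poses for a robot goal marker (BP_GoalRobot).
; BeginPlay binds a command listener whose handler is empty.
; Pose helpers are meant to compose offsets with the user's head pose, relative to an anchored BP_RoomBase or the game mode, then print and move the marker.
; Room-search loops and anchor math are disconnected, including in NavIntent, leaving those calculations unfinished.
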(event `self.ReceiveBeginPlay`
  (`self.cmd`)
  (`self.navigation_cmd`))

(event `cmd`
  (add `self.WaitForCommand` (delegate `OnCommandReceived`)))

(event `OnCommandReceived`)

(event `navigation_cmd`)

(event `NavIntent`
  (params (xGoal :type Integer) (yGoal :type Integer))
  (bind _outactors (`GameplayStatics.GetAllActorsOfClass` "/Game/Representations/Map_Representations/BP_RoomBase.BP_RoomBase_C")))

(event `self.ReceiveTick`
  (params (DeltaSeconds :type "Float (single-precision)")))

(fn `Get Here Pose`
  (returns (Transform :type "Transform Structure"))
  (bind (_location _rotation) (`self.GetLocationOfP_WRT_Anchor` 20.0))
  (bind _returnvalue (`KismetMathLibrary.MakeTransform` _location _rotation))
  (`KismetSystemLibrary.PrintString` (`KismetStringLibrary.Conv_TransformToString` _returnvalue) true true (struct :`R` 0.973907 :`G` 1.0 :`B` 0.15 :`A` 1.0) 10.0)
  (bind _translation (`self.Get Location Of P WRT Game Mode` (0.0 0.0 0.0)))
  (bind _returnvalue_2 (`GameplayStatics.GetActorOfClass` "/Game/FabianTest/Blueprint/Pawn/BP_GoalRobot.BP_GoalRobot_C"))
  (`self.K2_SetActorLocation` _returnvalue_2 (`KismetMathLibrary.MakeVector` (.x _translation) (.y _translation) -150.0) false false)
  (return _returnvalue))

(fn `Get Location Of P WRT Game Mode`
  (params (InputTranslation :type "Vector Structure") (InputRotation :type "Rotator Structure"))
  (returns (Translation :type "Vector Structure") (Rotation :type "Rotator Structure"))
  (bind _outactors (`GameplayStatics.GetAllActorsOfClass` "/Game/Representations/Map_Representations/BP_RoomBase.BP_RoomBase_C")))

(fn `Get There Pose`
  (returns (Transform :type "Transform Structure"))
  (bind (_location_x _location_y _location_z) (`KismetMathLibrary.BreakVector` (`self.Location`)))
  (bind (_rotation_roll _rotation_pitch _rotation_yaw) (`KismetMathLibrary.BreakRotator` (`self.Rotation`)))
  (bind (_location _rotation) (`self.GetLocationOfP_WRT_Anchor` _location_x _location_y _location_z _rotation_yaw))
  (bind _returnvalue (`KismetMathLibrary.MakeTransform` _location _rotation))
  (`KismetSystemLibrary.PrintString` (`KismetStringLibrary.Conv_TransformToString` _returnvalue) true true (struct :`R` 0.973907 :`G` 1.0 :`B` 0.15 :`A` 1.0) 10.0)
  (bind _translation (`self.Get Location Of P WRT Game Mode` (`self.Location`) (`self.Rotation`)))
  (bind _returnvalue_2 (`GameplayStatics.GetActorOfClass` "/Game/FabianTest/Blueprint/Pawn/BP_GoalRobot.BP_GoalRobot_C"))
  (`self.K2_SetActorLocation` _returnvalue_2 (`KismetMathLibrary.MakeVector` (.x _translation) (.y _translation) -150.0) false false)
  (return _returnvalue))

(fn `getHereCmd`
  (returns (ReturnValue :type "Transform Structure"))
  (bind _transform (`self.Get Here Pose`))
  (return))

(fn `GetLocationOfP_WRT_Anchor`
  (params (x :type "Float (double-precision)") (y :type "Float (double-precision)") (z :type "Float (double-precision)") (theta :type "Float (double-precision)"))
  (returns (Location :type "Vector Structure") (Rotation :type "Rotator Structure"))
  (bind _outactors (`GameplayStatics.GetAllActorsOfClass` "/Game/Representations/Map_Representations/BP_RoomBase.BP_RoomBase_C")))

(fn `getThereCmd`
  (`self.Get There Pose`)
  (return))

(fn `UserConstructionScript`)