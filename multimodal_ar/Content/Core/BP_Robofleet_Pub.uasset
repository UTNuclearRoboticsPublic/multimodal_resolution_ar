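; Robofleet publisher that reports a HoloLens wearer to ROS as an "operator" agent, using a randomly suffixed name and callsign.
; Looping timers publish status, head-pose odometry and anchor-relative TF.
; A delayed Tick picks the nearest BP_RoomBase anchor, which supplies the reported location and TF parent frame once localized.
; Positions convert from centimeters to meters with Y flipped for right-handed coordinates; TF yaw is also negated.
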(event `SetDebugOptions`
  (params (IsDebugPrintScreen :type Boolean) (IsDebugPrintLog :type Boolean))
  (set `self.IsDebugPrintScreen` IsDebugPrintScreen)
  (set `self.IsDebugPrintLog` IsDebugPrintLog))

(event `self.ReceiveBeginPlay`
  ;[1 1 1] Event Begin Play: Publish Status and Location
  (`self.SetDebugOptions` false)
  (`self.SetupName`)
  (`self.PublishOdometry`)
  (`self.PublishStatusMessage`)
  (`FileIO.WriteStringToProjectConfigFile` "ROBOFLEET" "MultimodalSettings" "ROS_NAMESPACE_TEMP" (`self.Device Name`))
  (`KismetSystemLibrary.PrintString` (`KismetStringLibrary.Conv_NameToString` (`HeadMountedDisplayFunctionLibrary.GetHMDDeviceName`)) (`self.IsDebugPrintScreen`) (`self.IsDebugPrintLog`))
  (`self.PublishTF_Setup`))

(event `PublishStatusMessage`
  ;[1 1 1] Publish Status
  (`KismetSystemLibrary.K2_SetTimerDelegate` (delegate `StatusRateLimit`) 2.0 true))

(event `StatusRateLimit`
  (bind _device_name (`self.Device Name`))
  (bind _batterylevel (`self.BatteryLevel`))
  ;[1 1 1] Publish Status
  (set `self.RobotStatusStruct` (make `RobotStatus` (`self.Status`) (`self.IsOk`) _batterylevel (`self.Location`)))
  (`RobofleetBPFunctionLibrary.PublishAgentStatusMsg` _device_name (make `AgentStatus` _device_name "operator" (`self.Callsign`) _batterylevel "" "working")))

(event `PublishOdometry`
  ;[1 1 1] Publish Odometry
  (`KismetSystemLibrary.K2_SetTimerDelegate` (delegate `OdomRate`) 0.1 true))

(event `OdomRate`
  (bind _returnvalue (`UxtFunctionLibrary.GetHeadPose`))
  (bind _device_name (`self.Device Name`))
  (bind (_returnvalue_x _returnvalue_y _returnvalue_z) (`KismetMathLibrary.BreakVector` (/ (.location _returnvalue) 100.0)))
  ;[1 1 1] Publish Odometry
  (`RobofleetBPFunctionLibrary.PublishTransformWithCovarianceStampedMsg` "odometry" (make `TransformWithCovarianceStamped` (make `TransformStamped` (make `Header` 0 (struct) (`KismetStringLibrary.Concat_StrStr` _device_name "/odom")) (`KismetStringLibrary.Concat_StrStr` _device_name "/base_link") (`KismetMathLibrary.MakeTransform` (`KismetMathLibrary.MakeVector` _returnvalue_x (* _returnvalue_y -1.0) _returnvalue_z) (`KismetMathLibrary.MakeRotator` (.roll (.rotation _returnvalue)) (.pitch (.rotation _returnvalue)) (.yaw (.rotation _returnvalue))))) (`self.OdometryCovariance`))))

(event `self.ReceiveTick`
  (params (DeltaSeconds :type "Float (single-precision)"))
  ;[1 1 1] Anchor Distance Check: Continuously Check For Anchors and How Far Hololens is From Anchor
  (`KismetSystemLibrary.Delay` 5.0)
  (bind _outactors (`GameplayStatics.GetAllActorsOfClass` "/Game/Representations/Map_Representations/BP_RoomBase.BP_RoomBase_C"))
  (bind _returnvalue (`KismetArrayLibrary.Array_Length` _outactors))
  (`KismetSystemLibrary.PrintString` (`KismetStringLibrary.Concat_StrStr` "Number of Room Base Actors Found: " (`KismetStringLibrary.Conv_IntToString` _returnvalue)) (`self.IsDebugPrintScreen`) (`self.IsDebugPrintLog`))
  (if (!= _returnvalue 0)
    (bind _outputpin (`self.GetClosestAnchor` _outactors))
    (bind _output_get (set `self.ClosestRoomBaseAnchor` _outputpin))
    (set `self.IsLocalizedToAnchor` true)
    (bind _representation_id (`/Game/Representations/Map_Representations/BP_AnchoredRepresentationBase.Representation ID` _output_get))
    (set `self.RoomBaseName` _representation_id)
    (`KismetSystemLibrary.PrintString` (`KismetStringLibrary.Concat_StrStr` "Closest Room Base: " _representation_id) (`self.IsDebugPrintScreen`) (`self.IsDebugPrintLog`))
    (else
      (`KismetSystemLibrary.PrintString` "No Anchors To Localize To" (`self.IsDebugPrintScreen`) (`self.IsDebugPrintLog`)))))

(event `SetupName`
  ;[1 1 1] Setup Name
  (set `self.RandomInt` (`KismetMathLibrary.RandomInteger` 5000))
  (`|ExecutionSequence`
    (:`then_0`
      (bind _value (`FileIO.ReadStringFromProjectConfigFile` "Robofleet" "MultimodalSettings" "ROS_NAMESPACE"))
      (set `self.Device Name` (`KismetStringLibrary.Concat_StrStr` _value (`KismetStringLibrary.Conv_IntToString` (`self.RandomInt`)))))
    (:`then_1`
      (bind _output_get (set `self.Callsign` (`KismetStringLibrary.Concat_StrStr` "U" (`KismetStringLibrary.Conv_IntToString` (`self.RandomInt`)))))
      (`FileIO.WriteStringToProjectConfigFile` "Robofleet" "MultimodalSettings" "CALLSIGN" _output_get))))

(event `PublishTF_Setup`
  ;[1 1 1] Publish hololens frame wrt anchor
  (`KismetSystemLibrary.K2_SetTimerDelegate` (delegate `CustomEvent`) 0.1 true))

(event `CustomEvent`
  (bind _closestroombaseanchor (`self.ClosestRoomBaseAnchor`))
  ;[1 1 1] Publish hololens frame wrt anchor
  (if (`self.IsLocalizedToAnchor`)
    (set `self.Status` "Localized")
    (set `self.Location` (`self.RoomBaseName`))
    (if (`KismetSystemLibrary.IsValid` _closestroombaseanchor)
      (bind (_returnvalue_x _returnvalue_y _returnvalue_z _returnvalue_theta) (`self.GetLocationDataFromClosestAnchor` _closestroombaseanchor))
      (`KismetArrayLibrary.Array_Add` (`self.TFArray`) (make `TransformStamped` (make `Header` 0 (struct) (`KismetStringLibrary.Concat_StrStr` "anchor_" (`KismetStringLibrary.Replace` (`self.RoomBaseName`) "-" "_"))) (`KismetStringLibrary.Concat_StrStr` (`self.Device Name`) "/base_link") (`KismetMathLibrary.MakeTransform` (`KismetMathLibrary.MakeVector` _returnvalue_x (* _returnvalue_y -1.0) _returnvalue_z) (`KismetMathLibrary.MakeRotator` 0.0 0.0 (* -1 _returnvalue_theta)))))
      (`RobofleetBPFunctionLibrary.PublishTFMessageMsg` (make `TFMessage` (`self.TFArray`)))
      (`KismetArrayLibrary.Array_Clear` (`self.TFArray`)))))

(fn `GetClosestAnchor`
  (params (Anchors :type "Array of /Game/Representations/Map_Representations/BP_RoomBase Object Reference"))
  (returns (OutputPin :type "/Game/Representations/Map_Representations/BP_RoomBase Object Reference"))
  (locals (Distance :type "Float (double-precision)") (Solution :type "/Game/Representations/Map_Representations/BP_RoomBase Object Reference"))
  (bind _output (`|GetArrayItem` Anchors))
  (if (`KismetSystemLibrary.IsValid` _output)
    (bind _distancefromanchor (`self.GetDistanceFromAnchor` _output))
    (set `self.ShortestDistance` _distancefromanchor)
    (set `local.Solution` _output)
    (for _array_element Anchors
      (bind _distancefromanchor_2 (`self.GetDistanceFromAnchor` _array_element (`self.IsDebugPrintScreen`) (`self.IsDebugPrintLog`)))
      (if (< _distancefromanchor_2 (`self.ShortestDistance`))
        (set `self.ShortestDistance` _distancefromanchor_2)
        (bind _output_get (set `local.Solution` _array_element))
        (`self.ClosestRoomBaseAnchorFound` _output_get)))
    (return (`local.Solution`))))

(fn `GetDistanceFromAnchor`
  (params (BP_RoomBaseRef :type "/Game/Representations/Map_Representations/BP_RoomBase Object Reference") (bPrintToScreen :type Boolean) (bPrintToLog :type Boolean))
  (returns (DistanceFromAnchor :type "Float (double-precision)"))
  (bind _returnvalue_location (`KismetMathLibrary.BreakTransform` (`UxtFunctionLibrary.GetHeadPose`)))
  (bind _returnvalue (`KismetMathLibrary.Vector_Distance` _returnvalue_location (`self.K2_GetActorLocation` BP_RoomBaseRef)))
  (`KismetSystemLibrary.PrintString` (`KismetStringLibrary.Concat_StrStr` "Distance from " (`/Game/Representations/Map_Representations/BP_AnchoredRepresentationBase.Representation ID` BP_RoomBaseRef) ": " (`KismetStringLibrary.Conv_DoubleToString` _returnvalue)) bPrintToScreen bPrintToLog)
  (return _returnvalue))

(fn `GetLocationDataFromClosestAnchor`
  (params (InputPin :type "/Game/Representations/Map_Representations/BP_RoomBase Object Reference"))
  (returns (ReturnValue_X :type "Float (double-precision)") (ReturnValue_Y :type "Float (double-precision)") (ReturnValue_Z :type "Float (double-precision)") (ReturnValue_Theta :type "Float (double-precision)"))
  (bind (_returnvalue_location _returnvalue_rotation) (`KismetMathLibrary.BreakTransform` (`UxtFunctionLibrary.GetHeadPose`)))
  (bind _returnvalue (`KismetMathLibrary.NegateRotator` (`self.K2_GetActorRotation` InputPin)))
  (bind _returnvalue_2 (`KismetMathLibrary.GreaterGreater_VectorRotator` (- _returnvalue_location (`self.K2_GetActorLocation` InputPin)) _returnvalue))
  (bind (_returnvalue_roll _returnvalue_pitch _returnvalue_yaw) (`KismetMathLibrary.BreakRotator` (`KismetMathLibrary.ComposeRotators` _returnvalue_rotation _returnvalue)))
  (bind (_returnvalue_x _returnvalue_y _returnvalue_z) (`KismetMathLibrary.BreakVector` (/ _returnvalue_2 100.0)))
  (`KismetSystemLibrary.PrintString` (`KismetStringLibrary.Conv_VectorToString` _returnvalue_2) false false)
  (return _returnvalue_x _returnvalue_y _returnvalue_z _returnvalue_yaw))

(fn `UserConstructionScript`
  (`parent.UserConstructionScript`))