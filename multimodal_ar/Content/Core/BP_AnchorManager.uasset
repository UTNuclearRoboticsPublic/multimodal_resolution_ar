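; Manager actor that resolves Azure Spatial Anchors in mixed reality and shares them through Robofleet.
; Anchor IDs from the client's new-anchor event are queued and located one watcher at a time.
; Located anchors spawn a BP_RoomBase pinned to an AR pin, then publish an anchor message and a head-pose measurement relative to that actor.
; Anchors saved to the cloud are submitted to the AugRE database with representation ID and timestamp.
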(event `SetDebugOptions`
  (params (IsDebugPrintScreen :type Boolean) (IsDebugPrintLog :type Boolean))
  ;[1 1 1] Debug Settings
  (set `self.IsDebugPrintScreen` IsDebugPrintScreen)
  (set `self.IsDebugPrintLog` IsDebugPrintLog))

(event `self.ReceiveBeginPlay`
  ;[1 1 1] Event Begin Play: Request Anchor ID from ASA Database and Create Watcher with Watcher ID
  (`self.SetDebugOptions` true true)
  (`self.StartListeningToAzureSpatialAnchorDelegate`)
  (`self.SetupASADelegates`)
  (`KismetSystemLibrary.Delay` 4.0)
  (bind _returnvalue (`RobofleetBPFunctionLibrary.GetClientReference`))
  (add `RobofleetBase.OnNewAnchorSeen` _returnvalue (delegate `OnNewAnchorSeen_Event_0`)))

(event `OnNewAnchorSeen_Event_0`
  (params (AsaId :type String))
  ;[1 1 1] Event Begin Play: Request Anchor ID from ASA Database and Create Watcher with Watcher ID
  (bind _output_get (set `self.AsaId` AsaId))
  (`KismetSystemLibrary.PrintString` (`KismetStringLibrary.Concat_StrStr` "[Anchor Manager] OnNewAnchorSeen: AsaID= " AsaId) (`self.IsDebugPrintScreen`) (`self.IsDebugPrintLog`) (struct :`G` 0.66 :`B` 1.0 :`A` 1.0) 10.0)
  (`KismetArrayLibrary.Array_Add` (`self.ListOfAnchors`) _output_get)
  (`KismetSystemLibrary.Delay` 2.0) ; NEED TO FIND A BETTER WAY
  (if (not (`self.isWatcherRunning`))
    (`self.CreateNewSessionWatcher` (`|MakeArray` (`|GetArrayItem` (`self.ListOfAnchors`))))))

(event `StartListeningToAzureSpatialAnchorDelegate`
  ;[1 1 1] Logic When Anchor is Found
  (add `AzureSpatialAnchorsEventComponent.ASAAnchorLocatedDelegate` (`self.AzureSpatialAnchorsEvent`) (delegate `OnAnchorFound`)))

(event `OnAnchorFound`
  (params (WatcherIdentifier :type Integer) (Status :type "EAzureSpatialAnchorsLocateAnchorStatus Enum" :default "AlreadyTracked") (CloudSpatialAnchor :type "AzureCloudSpatialAnchor Object Reference"))
  (bind (_returnvalue_location _returnvalue_rotation) (`KismetMathLibrary.BreakTransform` (`UxtFunctionLibrary.GetHeadPose`)))
  (bind _returnvalue (`AzureCloudSpatialAnchor.GetAppProperties` CloudSpatialAnchor))
  (bind _isdebugprintlog (`self.IsDebugPrintLog`))
  (bind _isdebugprintscreen (`self.IsDebugPrintScreen`))
  (bind _isdebugprintscreen_2 (`self.IsDebugPrintScreen`))
  (bind _isdebugprintlog_2 (`self.IsDebugPrintLog`))
  (bind (_value _returnvalue_2) (`BlueprintMapLibrary.Map_Find` (`self.AnchorAppProperties`) "Representation ID"))
  ;[1 1 1] Logic When Anchor is Found
  (`KismetSystemLibrary.PrintString` "[Anchor Manager] ASAAnchor Located Delegate" (`self.IsDebugPrintScreen`) (`self.IsDebugPrintLog`))
  (`KismetSystemLibrary.PrintString` (`KismetStringLibrary.Conv_IntToString` (`KismetArrayLibrary.Array_Length` (`self.ListOfAnchors`))) (`self.IsDebugPrintScreen`) (`self.IsDebugPrintLog`))
  (`|ExecutionSequence`
    (:`then_0`
      (`self.Print app properties` _returnvalue (`AzureCloudSpatialAnchor.GetAzureCloudIdentifier` CloudSpatialAnchor))
      (set `self.AnchorAppProperties` _returnvalue)
      (switch `EAzureSpatialAnchorsLocateAnchorStatus` Status
        (:`AlreadyTracked`
          (`KismetSystemLibrary.PrintString` "[AnchorStatus] Already Tracked"))
        (:`Located`
          (`|ExecutionSequence`
            (:`then_0`
              (if _returnvalue_2
                (set `self.Pin ID` _value)
                (else
                  (set `self.Pin ID` (`KismetStringLibrary.Concat_StrStr` "O_" (`KismetStringLibrary.Conv_DoubleToString` (`KismetMathLibrary.RandomFloat`)))))))
            (:`then_1`
              (bind _constructed_object (`self.Spawn Anchored Representation From ASA` (`self.AnchorAppProperties`) (`self.Pin ID`)))
              (bind (_outarpin _returnvalue_3) (`AzureSpatialAnchorsLibrary.CreateARPinAroundAzureCloudSpatialAnchor` (`self.Pin ID`) CloudSpatialAnchor))
              (if _returnvalue_3
                (`KismetSystemLibrary.PrintString` "ARPIN created succesfully from cloud Anchor" _isdebugprintscreen_2 _isdebugprintlog_2)
                (`ARBlueprintLibrary.PinComponentToARPin` (`/Game/Representations/Map_Representations/BP_AnchoredRepresentationBase.DefaultSceneRoot` _constructed_object) _outarpin)
                (`self.Publish Anchor Msg` (`ARPin.GetLocalToWorldTransform` _outarpin) (`self.Pin ID`))
                (bind _returnvalue_4 (`GameplayStatics.GetActorOfClass` "/Game/Core/BP_Robofleet_Pub.BP_Robofleet_Pub_C"))
                (bind _returnvalue_5 (`self.K2_GetActorRotation` _constructed_object))
                (bind (_returnvalue_x _returnvalue_y _returnvalue_z) (`KismetMathLibrary.BreakVector` (/ (`KismetMathLibrary.GreaterGreater_VectorRotator` (- _returnvalue_location (`self.K2_GetActorLocation` _constructed_object)) (`KismetMathLibrary.NegateRotator` _returnvalue_5)) 100.0)))
                (bind (_returnvalue_roll _returnvalue_pitch _returnvalue_yaw) (`KismetMathLibrary.BreakRotator` (`KismetMathLibrary.ComposeRotators` _returnvalue_rotation _returnvalue_5)))
                (`RobofleetBPFunctionLibrary.PublishTransformWithCovarianceStampedMsg` "measurements" (make `TransformWithCovarianceStamped` (make `TransformStamped` (make `Header` 0 (struct) (`KismetStringLibrary.Concat_StrStr` "anchor_" (`/Game/Representations/Map_Representations/BP_AnchoredRepresentationBase.Representation ID` _constructed_object))) (`KismetStringLibrary.Concat_StrStr` (`/Game/Core/BP_Robofleet_Pub.Device Name` _returnvalue_4) "/base_link") (`KismetMathLibrary.MakeTransform` (`KismetMathLibrary.MakeVector` _returnvalue_x _returnvalue_y _returnvalue_z) (`KismetMathLibrary.MakeRotator` 0.0 0.0 _returnvalue_yaw))) (`self.measurementCov`)))
                (else
                  (`KismetSystemLibrary.PrintString` "ARPIN CANNOT be created from cloud anchor" _isdebugprintscreen_2 _isdebugprintlog_2))))))
        (:`NotLocated`
          (`KismetSystemLibrary.PrintString` "[AnchorStatus] Not Located"))
        (:`NotLocatedAnchorDoesNotExist`
          (`KismetSystemLibrary.PrintString` (`KismetStringLibrary.Concat_StrStr` "Anchor Does Not Exist: ")))))
    (:`then_1`
      (`KismetArrayLibrary.Array_Remove` (`self.ListOfAnchors`))
      (`AzureSpatialAnchorsLibrary.StopWatcher` (`self.LastAsaWatcherId`))
      (set `self.isWatcherRunning` false)
      (`|ExecutionSequence`
        (:`then_0`
          (if (> (`KismetArrayLibrary.Array_Length` (`self.ListOfAnchors`)) 0)
            (`self.CreateNewSessionWatcher` (`|MakeArray` (`|GetArrayItem` (`self.ListOfAnchors`))))))
        (:`then_1`
          (if (or _isdebugprintscreen _isdebugprintlog)
            (for _array_element (`self.ListOfAnchors`)
              (`KismetSystemLibrary.PrintString` (`KismetStringLibrary.Concat_StrStr` "Still Need to Find: " _array_element) _isdebugprintscreen _isdebugprintlog))))))))

(event `SetupASADelegates`
  ;[1 1 1] Submit Azure Entry to AugREDatabase
  (bind _asmrgame_mode (cast `/Game/Core/MRGameMode` (`GameplayStatics.GetGameMode`)))
  (add `/Game/Core/MRGameMode.ASA Saved To Cloud` _asmrgame_mode (delegate `ASA saved to cloud handler`)))

(event `ASA saved to cloud handler`
  (params (`Azure Cloud Identifier` :type String) (`Representation ID` :type String))
  ;[1 1 1] Submit Azure Entry to AugREDatabase
  (`self.SubmitDatabaseEntry` `Representation ID` `Azure Cloud Identifier` (`KismetMathLibrary.UtcNow`))
  (`KismetSystemLibrary.PrintString` (`KismetStringLibrary.Concat_StrStr` "Submit Database Entry:" "asa_id: " `Azure Cloud Identifier` "Rep_id" `Representation ID`) (`self.IsDebugPrintScreen`) (`self.IsDebugPrintLog`)))

(fn `CreateNewSessionWatcher`
  (params (ListOfAnchors :type "Array of String (by ref)"))
  (bind _isdebugprintscreen (`self.IsDebugPrintScreen`))
  (bind _isdebugprintlog (`self.IsDebugPrintLog`))
  (for _array_element ListOfAnchors
    (`KismetSystemLibrary.PrintString` _array_element))
  (bind (_outwatcheridentifier _outresult _outerrorstring) (`AzureSpatialAnchorsLibrary.CreateWatcher` (make `AzureSpatialAnchorsLocateCriteria` false ListOfAnchors)))
  (`KismetSystemLibrary.PrintString` (`KismetStringLibrary.Concat_StrStr` "New Watcher Created [" "# " (`KismetStringLibrary.Conv_IntToString` _outwatcheridentifier) "]") _isdebugprintscreen _isdebugprintlog)
  (`KismetSystemLibrary.PrintString` _outerrorstring _isdebugprintscreen _isdebugprintlog)
  (set `self.LastAsaWatcherId` _outwatcheridentifier)
  (set `self.isWatcherRunning` true))

(fn `GetRepIdFromAsaID`
  (params (Target :type "AzureCloudSpatialAnchor Object Reference") (TargetMap :type "Map of String to String (by ref)"))
  (bind _returnvalue (`AzureCloudSpatialAnchor.GetAzureCloudIdentifier` Target))
  (bind _keys (`BlueprintMapLibrary.Map_Keys` TargetMap))
  (for _array_element _keys
    (if (`KismetStringLibrary.EqualEqual_StrStr` (`BlueprintMapLibrary.Map_Find` TargetMap _array_element) _returnvalue)
      (`KismetSystemLibrary.PrintString` (`KismetStringLibrary.Concat_StrStr` "RepID:" _array_element "; AsaID: " _returnvalue))
      (else
        (`KismetSystemLibrary.PrintString` (`KismetStringLibrary.Concat_StrStr` "Get Azure Cloud Identifier" _returnvalue))))))

(fn `Print app properties`
  (params (TargetMap :type "Map of String to String (by ref)") (`target id` :type "String (by ref)"))
  (locals (`Spawn Scale` :type "Vector Structure") (OutputObject :type Boolean))
  (bind _isdebugprintscreen (`self.IsDebugPrintScreen`))
  (bind _isdebugprintlog (`self.IsDebugPrintLog`))
  (`KismetSystemLibrary.PrintString` `target id`)
  (`KismetSystemLibrary.PrintString` (`KismetStringLibrary.Concat_StrStr` "Lengt of App Properties: " (`KismetStringLibrary.Conv_IntToString` (`BlueprintMapLibrary.Map_Length` TargetMap))) (`self.IsDebugPrintScreen`) (`self.IsDebugPrintLog`))
  (`KismetSystemLibrary.PrintString` "KEYS APP PROPERTIES")
  (bind _keys (`BlueprintMapLibrary.Map_Keys` TargetMap))
  (for _array_element _keys
    (`KismetSystemLibrary.PrintString` _array_element _isdebugprintscreen _isdebugprintlog))
  (`KismetSystemLibrary.PrintString` "VALUES" _isdebugprintscreen _isdebugprintlog)
  (bind _values (`BlueprintMapLibrary.Map_Values` TargetMap))
  (for _array_element_2 _values
    (`KismetSystemLibrary.PrintString` _array_element_2)))

(fn `Publish Anchor Msg`
  (params (Transform :type "Transform Structure") (RepId :type String))
  (bind _value (`BlueprintMapLibrary.Map_Find` (`self.ListOfAnchorsFoundInDb`) RepId))
  (bind _value_2 (`FileIO.ReadStringFromProjectConfigFile` "Robofleet" "MultimodalSettings" "ROS_NAMESPACE"))
  (`RobofleetBPFunctionLibrary.PublishAzureSpatialAnchorMsg` _value_2 (make `AzureSpatialAnchor` _value RepId "" (struct) (make `PoseWithCovarianceStamped` (struct :`stamp` (struct)) (make `PoseWithCovariance` Transform))))
  (`KismetSystemLibrary.PrintString` (`KismetStringLibrary.Concat_StrStr` "Anchor Msg Sent!" "; AsaId: " _value "; RepId:" RepId) (`self.IsDebugPrintScreen`) (`self.IsDebugPrintLog`)))

(fn `Spawn Anchored Representation From ASA`
  (params (Properties :type "Map of String to String") (pin_id :type String))
  (returns (`Constructed Object` :type "/Game/Representations/Map_Representations/BP_AnchoredRepresentationBase Object Reference"))
  (locals (`Spawn Scale` :type "Vector Structure" :default (1.0 1.0 1.0)) (OutputObject :type Boolean) (NewLocalVar_0 :type String :default "Representation ID"))
  (bind _output (`|GetArrayItem` (`self.ListOfAnchors`)))
  (bind _returnvalue (`|SpawnActorFromClass` "/Game/Representations/Map_Representations/BP_RoomBase.BP_RoomBase_C" (`KismetMathLibrary.MakeTransform` (0.0 0.0 0.0) (struct) (`local.Spawn Scale`)) "Undefined" "OverrideRootScale" null _output _output true null))
  (return _returnvalue))

(fn `UserConstructionScript`)